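; Basic enemy Blueprint that detects the player by distance and deals damage at close range.
; Tick sets the PlayerInRange blackboard key from the distance to the player.
; When close, a forward Pawn line trace gates a delayed ApplyDamage on the player, whichever pawn it hits.
; An unconnected, never-executed chain holds timed health reduction and an AI health update call.
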(event `self.ReceiveTick`
  (params (DeltaSeconds :type "Float (single-precision)"))
  (bind _returnvalue (`KismetStringLibrary.Conv_StringToName` "PlayerInRange"))
  (bind _returnvalue_2 (`AIBlueprintHelperLibrary.GetBlackboard` null))
  (bind _returnvalue_3 (`self.K2_GetActorLocation`))
  ;[1 1 1] Set PlayerInRange
  (`/Engine/EditorBlueprintResources/StandardMacros.CompareFloat` (`self.GetDistanceTo` self (`GameplayStatics.GetPlayerCharacter` 0)) 600.0
    (:`>`
      (`BlackboardComponent.SetValueAsBool` _returnvalue_2 _returnvalue false))
    (:`==`
      (`BlackboardComponent.SetValueAsBool` _returnvalue_2 _returnvalue true :!label _label)
      ;[1 1 1] Attack when in range
      (`/Engine/EditorBlueprintResources/StandardMacros.CompareFloat` (`self.GetDistanceTo` self (`GameplayStatics.GetPlayerCharacter` 0)) 200.0
        (:`<`
          (bind (_outhit _returnvalue_4) (`KismetSystemLibrary.LineTraceSingleForObjects` _returnvalue_3 (+ _returnvalue_3 (* (`KismetMathLibrary.GetForwardVector` (`self.K2_GetActorRotation`)) 10000.0)) (`|MakeArray` "ObjectTypeQuery3" :!type "EObjectTypeQuery Enum")))
          (if _returnvalue_4
            (`KismetSystemLibrary.Delay` 1.0)
            (`GameplayStatics.ApplyDamage` (`GameplayStatics.GetPlayerCharacter` 0) 10.0)))))
    (:`<`
      (goto _label))))

(event `self.ReceiveBeginPlay`)

(fn `UserConstructionScript`)
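; Enemy AI controller that moves its controlled pawn back and forth between two patrol target points.
; BeginPlay fills PatrolPoints with every TargetPoint tagged patrol_point_1.
; The Patrol event chains AI MoveTo calls to the first two entries with a short pause after each, then calls itself to loop.
; Nothing in this graph starts Patrol, and a failed move ends the loop.
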(event `self.ReceiveBeginPlay`
  ;[1 1 1] Get patrol points
  (bind _outactors (`GameplayStatics.GetAllActorsOfClass` "/Script/Engine.TargetPoint"))
  (for _array_element _outactors
    (if (`self.ActorHasTag` _array_element "patrol_point_1")
      (`KismetArrayLibrary.Array_Add` (`self.Patrol Points`) _array_element))))

(event `Patrol`
  ;[1 1 1] Patrol
  (`|AIMoveTo` (`self.K2_GetPawn`) (0.0 0.0 0.0) (`|GetArrayItem` (`self.Patrol Points`))
    (:`OnSuccess`
      (`KismetSystemLibrary.Delay` 2.0)
      (`|AIMoveTo` (`self.K2_GetPawn`) (0.0 0.0 0.0) (`|GetArrayItem` (`self.Patrol Points`) 1)
        (:`OnSuccess`
          (`KismetSystemLibrary.Delay` 2.0)
          (`self.Patrol`))))))

(fn `UserConstructionScript`)